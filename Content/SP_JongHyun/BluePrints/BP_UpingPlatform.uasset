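; Moving platform Blueprint that shuttles its static mesh back and forth between two marker components, PosA and PosB.
; On BeginPlay the mesh snaps to PosA, then a self-repeating FlipFlop loop alternates eased MoveComponentTo calls toward PosB and PosA.
; MovingTime sets each trip's duration and PauseTime sets the delay before the next flip.
; The OnActive event is empty, so movement always starts automatically.
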(event Custom|OnActive)

(event EventBeginPlay
  ;[1 1 1] 플랫폼 위치 초기화
  (Transformation|SetWorldLocation (Variables|Default|GetStaticMesh) (Transformation|GetWorldLocation (Variables|Default|GetPosA)) false false)
  ;[1 1 1] 플랫폼 왔다갔다
  ;;[1 1 1] A,B번갈아 실행
  (Utilities|FlowControl|FlipFlop :!label _label
    (:A
      (Components|MoveComponentTo (Variables|Default|GetStaticMesh) (Variables|/Script/Engine.SceneComponent|GetRelativeLocation (Variables|Default|GetPosB)) "0, 0, 0" true true (Variables|Default|GetMovingTim,e) false))
    (:B
      (Components|MoveComponentTo (Variables|Default|GetStaticMesh) (Variables|/Script/Engine.SceneComponent|GetRelativeLocation (Variables|Default|GetPosA)) "0, 0, 0" true true (Variables|Default|GetMovingTim,e) false)))
  (Utilities|FlowControl|Delay (Variables|Default|GetPauseTime))
  (goto _label))

(fn ConstructionScript)
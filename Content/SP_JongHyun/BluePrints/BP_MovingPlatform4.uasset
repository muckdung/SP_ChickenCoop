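; BP_MovingPlatform4 is a moving platform that stays idle until something overlaps its BoxCollision.
; An overlap snaps the platform to PosA, then a FlipFlop alternates eased MoveComponentTo moves toward PosB and PosA over MovingTime.
; A Delay of PauseTime loops back into the FlipFlop for endless back-and-forth motion, with no guard against repeated overlaps.
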(event OnComponentBeginOverlap(BoxCollision)
  (params (OverlappedComponent :type Primitive%20Component%20Object%20Reference) (OtherActor :type Actor%20Object%20Reference) (OtherComp :type Primitive%20Component%20Object%20Reference) (OtherBodyIndex :type Integer) (bFromSweep :type Boolean) (SweepResult :type Hit%20Result%20Structure%20%28by%20ref%29))
  ;[1 1 1] 플랫폼 위치 초기화
  (Transformation|SetWorldLocation (Variables|Default|GetPlatform) (Transformation|GetWorldLocation (Variables|Default|GetPosA)) false false)
  ;[1 1 1] 플랫폼 왔다갔다
  ;;[1 1 1] A,B번갈아 실행
  (Utilities|FlowControl|FlipFlop :!label _label
    (:A
      (Components|MoveComponentTo (Variables|Default|GetPlatform) (Variables|/Script/Engine.SceneComponent|GetRelativeLocation (Variables|Default|GetPosB)) "0, 0, 0" true true (Variables|Default|GetMovingTime) false))
    (:B
      (Components|MoveComponentTo (Variables|Default|GetPlatform) (Variables|/Script/Engine.SceneComponent|GetRelativeLocation (Variables|Default|GetPosA)) "0, 0, 0" true true (Variables|Default|GetMovingTime) false)))
  (Utilities|FlowControl|Delay (Variables|Default|GetPauseTime))
  (goto _label))

(event Custom|OnActive)

(event EventBeginPlay)

(fn ConstructionScript)
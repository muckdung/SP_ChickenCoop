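; Walkable piano actor that plays a note when the player character steps on one of its keys.
; Thirteen box triggers each handle begin overlap, cast the other actor to BP_ThirdPersonCharacter, and play their own piano sound.
; Notes play as non-spatial 2D sounds, with each key wired separately rather than through shared logic.
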(event OnComponentBeginOverlap(Box7)
  (params (OverlappedComponent :type Primitive%20Component%20Object%20Reference) (OtherActor :type Actor%20Object%20Reference) (OtherComp :type Primitive%20Component%20Object%20Reference) (OtherBodyIndex :type Integer) (bFromSweep :type Boolean) (SweepResult :type Hit%20Result%20Structure%20%28by%20ref%29))
  (Utilities|Casting|CastToBP_ThirdPersonCharacter OtherActor)
  (Audio|PlaySound2D "/Game/SP_JongHyun/Sounds/Piano/FX_piano07.FX_piano07" 1.0 1.0 0.0 0 0))

(event OnComponentBeginOverlap(Box8)
  (params (OverlappedComponent :type Primitive%20Component%20Object%20Reference) (OtherActor :type Actor%20Object%20Reference) (OtherComp :type Primitive%20Component%20Object%20Reference) (OtherBodyIndex :type Integer) (bFromSweep :type Boolean) (SweepResult :type Hit%20Result%20Structure%20%28by%20ref%29))
  (Utilities|Casting|CastToBP_ThirdPersonCharacter OtherActor)
  (Audio|PlaySound2D "/Game/SP_JongHyun/Sounds/Piano/FX_piano08.FX_piano08" 1.0 1.0 0.0 0 0))

(event OnComponentBeginOverlap(Box9)
  (params (OverlappedComponent :type Primitive%20Component%20Object%20Reference) (OtherActor :type Actor%20Object%20Reference) (OtherComp :type Primitive%20Component%20Object%20Reference) (OtherBodyIndex :type Integer) (bFromSweep :type Boolean) (SweepResult :type Hit%20Result%20Structure%20%28by%20ref%29))
  (Utilities|Casting|CastToBP_ThirdPersonCharacter OtherActor)
  (Audio|PlaySound2D "/Game/SP_JongHyun/Sounds/Piano/FX_piano09.FX_piano09" 1.0 1.0 0.0 0 0))

(event OnComponentBeginOverlap(Box10)
  (params (OverlappedComponent :type Primitive%20Component%20Object%20Reference) (OtherActor :type Actor%20Object%20Reference) (OtherComp :type Primitive%20Component%20Object%20Reference) (OtherBodyIndex :type Integer) (bFromSweep :type Boolean) (SweepResult :type Hit%20Result%20Structure%20%28by%20ref%29))
  (Utilities|Casting|CastToBP_ThirdPersonCharacter OtherActor)
  (Audio|PlaySound2D "/Game/SP_JongHyun/Sounds/Piano/FX_piano10.FX_piano10" 1.0 1.0 0.0 0 0))

(event OnComponentBeginOverlap(Box11)
  (params (OverlappedComponent :type Primitive%20Component%20Object%20Reference) (OtherActor :type Actor%20Object%20Reference) (OtherComp :type Primitive%20Component%20Object%20Reference) (OtherBodyIndex :type Integer) (bFromSweep :type Boolean) (SweepResult :type Hit%20Result%20Structure%20%28by%20ref%29))
  (Utilities|Casting|CastToBP_ThirdPersonCharacter OtherActor)
  (Audio|PlaySound2D "/Game/SP_JongHyun/Sounds/Piano/FX_piano11.FX_piano11" 1.0 1.0 0.0 0 0))

(event OnComponentBeginOverlap(Box12)
  (params (OverlappedComponent :type Primitive%20Component%20Object%20Reference) (OtherActor :type Actor%20Object%20Reference) (OtherComp :type Primitive%20Component%20Object%20Reference) (OtherBodyIndex :type Integer) (bFromSweep :type Boolean) (SweepResult :type Hit%20Result%20Structure%20%28by%20ref%29))
  (Utilities|Casting|CastToBP_ThirdPersonCharacter OtherActor)
  (Audio|PlaySound2D "/Game/SP_JongHyun/Sounds/Piano/FX_piano12.FX_piano12" 1.0 1.0 0.0 0 0))

(event OnComponentBeginOverlap(Box13)
  (params (OverlappedComponent :type Primitive%20Component%20Object%20Reference) (OtherActor :type Actor%20Object%20Reference) (OtherComp :type Primitive%20Component%20Object%20Reference) (OtherBodyIndex :type Integer) (bFromSweep :type Boolean) (SweepResult :type Hit%20Result%20Structure%20%28by%20ref%29))
  (Utilities|Casting|CastToBP_ThirdPersonCharacter OtherActor)
  (Audio|PlaySound2D "/Game/SP_JongHyun/Sounds/Piano/FX_piano13.FX_piano13" 1.0 1.0 0.0 0 0))

(event OnComponentBeginOverlap(Box1)
  (params (OverlappedComponent :type Primitive%20Component%20Object%20Reference) (OtherActor :type Actor%20Object%20Reference) (OtherComp :type Primitive%20Component%20Object%20Reference) (OtherBodyIndex :type Integer) (bFromSweep :type Boolean) (SweepResult :type Hit%20Result%20Structure%20%28by%20ref%29))
  (Utilities|Casting|CastToBP_ThirdPersonCharacter OtherActor)
  (Audio|PlaySound2D "/Game/SP_JongHyun/Sounds/Piano/FX_piano01.FX_piano01" 1.0 1.0 0.0 0 0))

(event OnComponentBeginOverlap(Box2)
  (params (OverlappedComponent :type Primitive%20Component%20Object%20Reference) (OtherActor :type Actor%20Object%20Reference) (OtherComp :type Primitive%20Component%20Object%20Reference) (OtherBodyIndex :type Integer) (bFromSweep :type Boolean) (SweepResult :type Hit%20Result%20Structure%20%28by%20ref%29))
  (Utilities|Casting|CastToBP_ThirdPersonCharacter OtherActor)
  (Audio|PlaySound2D "/Game/SP_JongHyun/Sounds/Piano/FX_piano02.FX_piano02" 1.0 1.0 0.0 0 0))

(event OnComponentBeginOverlap(Box3)
  (params (OverlappedComponent :type Primitive%20Component%20Object%20Reference) (OtherActor :type Actor%20Object%20Reference) (OtherComp :type Primitive%20Component%20Object%20Reference) (OtherBodyIndex :type Integer) (bFromSweep :type Boolean) (SweepResult :type Hit%20Result%20Structure%20%28by%20ref%29))
  (Utilities|Casting|CastToBP_ThirdPersonCharacter OtherActor)
  (Audio|PlaySound2D "/Game/SP_JongHyun/Sounds/Piano/FX_piano03.FX_piano03" 1.0 1.0 0.0 0 0))

(event OnComponentBeginOverlap(Box4)
  (params (OverlappedComponent :type Primitive%20Component%20Object%20Reference) (OtherActor :type Actor%20Object%20Reference) (OtherComp :type Primitive%20Component%20Object%20Reference) (OtherBodyIndex :type Integer) (bFromSweep :type Boolean) (SweepResult :type Hit%20Result%20Structure%20%28by%20ref%29))
  (Utilities|Casting|CastToBP_ThirdPersonCharacter OtherActor)
  (Audio|PlaySound2D "/Game/SP_JongHyun/Sounds/Piano/FX_piano04.FX_piano04" 1.0 1.0 0.0 0 0))

(event OnComponentBeginOverlap(Box5)
  (params (OverlappedComponent :type Primitive%20Component%20Object%20Reference) (OtherActor :type Actor%20Object%20Reference) (OtherComp :type Primitive%20Component%20Object%20Reference) (OtherBodyIndex :type Integer) (bFromSweep :type Boolean) (SweepResult :type Hit%20Result%20Structure%20%28by%20ref%29))
  (Utilities|Casting|CastToBP_ThirdPersonCharacter OtherActor)
  (Audio|PlaySound2D "/Game/SP_JongHyun/Sounds/Piano/FX_piano05.FX_piano05" 1.0 1.0 0.0 0 0))

(event OnComponentBeginOverlap(Box6)
  (params (OverlappedComponent :type Primitive%20Component%20Object%20Reference) (OtherActor :type Actor%20Object%20Reference) (OtherComp :type Primitive%20Component%20Object%20Reference) (OtherBodyIndex :type Integer) (bFromSweep :type Boolean) (SweepResult :type Hit%20Result%20Structure%20%28by%20ref%29))
  (Utilities|Casting|CastToBP_ThirdPersonCharacter OtherActor)
  (Audio|PlaySound2D "/Game/SP_JongHyun/Sounds/Piano/FX_piano06.FX_piano06" 1.0 1.0 0.0 0 0))

(fn ConstructionScript)
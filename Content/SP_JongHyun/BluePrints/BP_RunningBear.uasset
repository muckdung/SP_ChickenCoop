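; BP_RunningBear is a bear hazard that charges when something overlaps its trigger box and damages the player character on contact.
; The box overlap plays a looping run animation while MoveComponentTo carries the skeletal mesh to PosA over MovingTime.
; The bear then switches to a walk animation, turns around and moves to PosB over ReturnTime.
; The mesh's own overlap applies damage to BP_ThirdPersonCharacter.
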(event OnComponentBeginOverlap(SkeletalMesh)
  (params (OverlappedComponent :type Primitive%20Component%20Object%20Reference) (OtherActor :type Actor%20Object%20Reference) (OtherComp :type Primitive%20Component%20Object%20Reference) (OtherBodyIndex :type Integer) (bFromSweep :type Boolean) (SweepResult :type Hit%20Result%20Structure%20%28by%20ref%29))
  (bind _asbp_third_person_character (Utilities|Casting|CastToBP_ThirdPersonCharacter OtherActor))
  (Game|Damage|ApplyDamage _asbp_third_person_character 1.0 0 0))

(event OnComponentBeginOverlap(Box)
  (params (OverlappedComponent :type Primitive%20Component%20Object%20Reference) (OtherActor :type Actor%20Object%20Reference) (OtherComp :type Primitive%20Component%20Object%20Reference) (OtherBodyIndex :type Integer) (bFromSweep :type Boolean) (SweepResult :type Hit%20Result%20Structure%20%28by%20ref%29))
  (Components|Animation|PlayAnimation (Variables|Default|GetSkeletalMesh) "/Game/SP_JongHyun/Bear_Animation/Fast_Run__1__Anim.Fast_Run__1__Anim" true)
  (Components|MoveComponentTo (Variables|Default|GetSkeletalMesh) (Variables|/Script/Engine.SceneComponent|GetRelativeLocation (Variables|Default|GetPosA)) "0, 0, 0" false false (Variables|Default|GetMovingTime) false)
  (Audio|Components|Audio|Stop (Variables|Default|GetSkeletalMesh))
  (Components|Animation|PlayAnimation (Variables|Default|GetSkeletalMesh) "/Game/SP_JongHyun/Bear_Animation/Walking_Anim.Walking_Anim" true)
  (Transformation|SetRelativeRotation (Variables|Default|GetSkeletalMesh) "0.000000,180.000000,0.000000" false false)
  (Components|MoveComponentTo (Variables|Default|GetSkeletalMesh) (Variables|/Script/Engine.SceneComponent|GetRelativeLocation (Variables|Default|GetPosB)) "0.000000,180.000000,0.000000" false false (Variables|Default|GetReturnTime) true))

(fn ConstructionScript)
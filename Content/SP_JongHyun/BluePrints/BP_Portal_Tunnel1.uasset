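; BP_Portal_Tunnel1 is a portal with a button that reveals it when the player character first touches the trigger sphere.
; The sphere's begin overlap accepts only BP_ThirdPersonCharacter, then sets the button's relative location to show the press, turns its material green and makes the portal and its Niagara effect visible.
; An IsActive flag is then set so the activation does not repeat; this Blueprint contains no teleport logic.
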(event OnComponentBeginOverlap(Sphere)
  (params (OverlappedComponent :type Primitive%20Component%20Object%20Reference) (OtherActor :type Actor%20Object%20Reference) (OtherComp :type Primitive%20Component%20Object%20Reference) (OtherBodyIndex :type Integer) (bFromSweep :type Boolean) (SweepResult :type Hit%20Result%20Structure%20%28by%20ref%29))
  ;[1 1 1] 버튼 눌리는거 표현
  (if (not (Variables|Default|GetIsActive))
    (Utilities|Casting|CastToBP_ThirdPersonCharacter OtherActor)
    (Utilities|FlowControl|Sequence
      (:then_0
        (Transformation|SetRelativeLocation (Variables|Default|GetButton) "0, 0, 0" false false)
        ;[1 1 1] 눌리면 버튼 색깔 바뀌기
        (Rendering|Material|SetMaterial (Variables|Default|GetButton) 0 "/AnimationSharing/AnimSharingGreen.AnimSharingGreen")
        (Rendering|SetVisibility (Variables|Default|GetPortal) true false))
      (:then_2
        (Variables|Default|SetIsActive true)))))

(fn ConstructionScript)
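; BP_UpDown is a moving platform that shuttles a crystal mesh back and forth between two arrow markers.
; From BeginPlay, a FlipFlop alternates eased MoveComponentTo moves toward ArrowB and ArrowA over MovingTime.
; A PauseTime delay follows each move and loops back into the FlipFlop, so the motion repeats indefinitely.
; An unconnected branch that would reset the mesh to PosA never runs.
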(event EventBeginPlay
  ;[1 1 1] 플랫폼 왔다갔다
  ;;[1 1 1] A,B번갈아 실행
  (Utilities|FlowControl|FlipFlop :!label _label
    (:A
      (Components|MoveComponentTo (Variables|Default|GetSM_crystal_flat_03) (Variables|/Script/Engine.SceneComponent|GetRelativeLocation (Variables|Default|GetArrowB)) "0, 0, 0" true true (Variables|Default|GetMovingTime) false))
    (:B
      (Components|MoveComponentTo (Variables|Default|GetSM_crystal_flat_03) (Variables|/Script/Engine.SceneComponent|GetRelativeLocation (Variables|Default|GetArrowA)) "0, 0, 0" true true (Variables|Default|GetMovingTime) false)))
  (Utilities|FlowControl|Delay (Variables|Default|GetPauseTime))
  (goto _label))

(fn ConstructionScript)
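; BP_Fan1 is a fan that pushes the player with wind, either always on or switched by linked interaction triggers.
; Triggers' interaction components feed an active count; reaching TriggersNeeded starts rotation and wind FX, while any switch-off stops them.
; Entering FanArea while active starts a looping timer that repeatedly launches the player along ForceDirection, weakening with distance, plus slight lift.
; Leaving the area clears the timer.
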(event OnComponentBeginOverlap(FanArea)
  (params (OverlappedComponent :type Primitive%20Component%20Object%20Reference) (OtherActor :type Actor%20Object%20Reference) (OtherComp :type Primitive%20Component%20Object%20Reference) (OtherBodyIndex :type Integer) (bFromSweep :type Boolean) (SweepResult :type Hit%20Result%20Structure%20%28by%20ref%29))
  (if (Variables|Default|GetActive)
    (bind _returnvalue (Utilities|Time|SetTimerbyEvent (delegate Custom|UpdateForce) 0.01 true))
    (Variables|Default|SetTimer _returnvalue)))

(event OnComponentEndOverlap(FanArea)
  (params (OverlappedComponent :type Primitive%20Component%20Object%20Reference) (OtherActor :type Actor%20Object%20Reference) (OtherComp :type Primitive%20Component%20Object%20Reference) (OtherBodyIndex :type Integer))
  (Utilities|Time|ClearandInvalidateTimerbyHandle (Variables|Default|GetTimer)))

(event Custom|OnInteract
  (params (On :type Boolean))
  (if On
    (bind _result (Math|Integer|IncrementInt (Variables|Default|GetTriggersActive))
      (:%20%20
        (if (>= _result (Variables|Default|GetTriggersNeeded))
          (CallFunction|StartFan))))
    (else
      (Variables|Default|SetTriggersActive (Math|Integer|Max(Integer) (- (Variables|Default|GetTriggersActive) 1)))
      (CallFunction|StopFan))))

(event Custom|StartFan
  ;[0.4565 0.8361 1] 팬 파티클 효과
  (Variables|Default|SetActive true)
  (Components|Activation|Activate (Variables|Default|GetFX_WindBands) true)
  (bind _rotationspeed (Timeline|FanRotation Play)
    (:Update
      (Transformation|AddLocalRotation (Variables|Default|GetFan) (Math|Rotator|MakeRotator _rotationspeed 0.0 0.0) false false))))

(event Custom|StopFan
  ;[0.4565 0.8361 1] 팬 파티클 효과
  (Variables|Default|SetActive false)
  (Components|Activation|Deactivate (Variables|Default|GetFX_WindBands))
  (bind _rotationspeed (Timeline|FanRotation Stop)
    (:Update
      (Transformation|AddLocalRotation (Variables|Default|GetFan) (Math|Rotator|MakeRotator _rotationspeed 0.0 0.0) false false))))

(event Custom|UpdateForce
  (bind _returnvalue (Game|GetPlayerCharacter 0))
  (if (Collision|IsOverlappingActor _returnvalue self :!class /Script/Engine.Actor)
    (Character|LaunchCharacter _returnvalue (+ (* (Math|Vector|GetForwardVector (Variables|Default|GetForceDirection)) (Math|Float|MapRangeClamped (Math|Vector|VectorLength (- (Transformation|GetActorLocation (Game|GetPlayerCharacter 0)) (Transformation|GetActorLocation))) 0.0 (* (.x (Variables|/Script/Engine.BoxComponent|GetBoxExtent (Variables|Default|GetFanArea))) 2.0) 8e+02 0.0)) "0,0,20.000000") false true)
    (else
      (Utilities|Time|ClearandInvalidateTimerbyHandle (Variables|Default|GetTimer)))))

(event EventBeginPlay
  (if (> (Utilities|Array|Length (Variables|Default|GetTriggers)) 0)
    (for _array_element (Variables|Default|GetTriggers)
      (EventDispatchers|AssignOnInteract (Actor|GetComponentbyClass _array_element "/Game/SP_JongHyun/AirFan/BP_InteractionComponent.BP_InteractionComponent_C") (delegate Custom|OnInteract))
      (CallFunction|StopFan))
    (else
      (CallFunction|StartFan))))

(fn ConstructionScript)
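; BP_NPC_Frog_001 is a frog NPC that shows a multi-line dialogue to the player through its Talk event.
; Each Talk call increments TalkIndex and writes that Dialogue entry into a WB_Dialogue_Frog widget, created on demand.
; While lines remain, it sets TalkOver on the player's BP_ThirdPersonCharacter and disables jumping.
; Past the last line it clears TalkOver, restores double jump and removes the widget, without resetting the index.
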(event EventTalk
  (bind _talkindex (Variables|Default|GetTalkIndex))
  (bind _asbp_third_person_character (Utilities|Casting|CastToBP_ThirdPersonCharacter (Game|GetPlayerCharacter 0)))
  (Variables|Default|SetAs%20BP%20Third%20Person%20Character _asbp_third_person_character)
  (Math|Integer|IncrementInt _talkindex
    (:%20%20
      (if (< _talkindex (Utilities|Array|Length (Variables|Default|Getdialogue)))
        (Variables|Default|GetNewVar
          (:then
            _)
          (:else
            (bind _returnvalue (Game|ConstructObjectfromClass (Game|GetPlayerController 0) "/Game/SP_MJ_ALL/SP_UI/SP_GameUI/WB_Dialogue_Frog.WB_Dialogue_Frog_C"))
            (bind _output_get (Variables|Default|SetNewVar _returnvalue))
            (UserInterface|Viewport|AddtoViewport _output_get 0)))
        (Rendering|Components|TextRender|SetText (Variables|/Game/SP_MJ_ALL/SP_UI/SP_GameUI/WB_Dialogue_Frog.WB_Dialogue_Frog_C|GetTalkText (Variables|Default|GetNewVar)) (Utilities|Text|ToText(String) (Utilities|Array|Get(acopy) (Variables|Default|Getdialogue) (Variables|Default|GetTalkIndex))))
        (Variables|/Game/ThirdPerson/Blueprints/BP_ThirdPersonCharacter.BP_ThirdPersonCharacter_C|SetTalkOver (Variables|Default|GetAs%20BP%20Third%20Person%20Character) true)
        (Variables|/Script/Engine.Character|SetJumpMaxCount (Variables|Default|GetAs%20BP%20Third%20Person%20Character) 0)
        (else
          (Variables|/Game/ThirdPerson/Blueprints/BP_ThirdPersonCharacter.BP_ThirdPersonCharacter_C|SetTalkOver (Variables|Default|GetAs%20BP%20Third%20Person%20Character) false)
          (Variables|/Script/Engine.Character|SetJumpMaxCount (Variables|Default|GetAs%20BP%20Third%20Person%20Character) 2)
          (Widget|RemovefromParent (Variables|Default|GetNewVar)))))))

(fn ConstructionScript)
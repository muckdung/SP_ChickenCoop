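; BP_Kangaroo is a talking NPC that leads the player into a timed, countdown-started activity.
; Each Talk call advances one of two dialogue arrays, selected by the player's Talkagain flag, in a reused WB_Dialogue_Frog widget while jumping is disabled.
; Both branches share an ending that restores jumping and, if TimerStart is unset, teleports the player to a fixed spot, disables input, shows WB_CountDown and closes the dialogue.
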(event EventTalk
  (bind _asbp_third_person_character (Utilities|Casting|CastToBP_ThirdPersonCharacter (Game|GetPlayerCharacter 0)))
  (bind _output_get (Variables|Default|SetAs%20BP%20Third%20Person%20Character _asbp_third_person_character))
  (if (Variables|/Game/ThirdPerson/Blueprints/BP_ThirdPersonCharacter.BP_ThirdPersonCharacter_C|GetTalkagain _output_get)
    (Math|Integer|IncrementInt (Variables|Default|GetTalkIndex_002)
      (:%20%20
        (if (< (Variables|Default|GetTalkIndex_002) (Utilities|Array|Length (Variables|Default|GetDialogue_002)))
          (Variables|Default|GetUI
            (:then
              _)
            (:else
              (bind _returnvalue (Game|ConstructObjectfromClass (Game|GetPlayerController 0) "/Game/SP_MJ_ALL/SP_UI/SP_GameUI/WB_Dialogue_Frog.WB_Dialogue_Frog_C"))
              (bind _output_get_2 (Variables|Default|SetUI _returnvalue))
              (UserInterface|Viewport|AddtoViewport _output_get_2 0)))
          (Rendering|Components|TextRender|SetText (Variables|/Game/SP_MJ_ALL/SP_UI/SP_GameUI/WB_Dialogue_Frog.WB_Dialogue_Frog_C|GetTalkText (Variables|Default|GetUI)) (Utilities|Text|ToText(String) (Utilities|Array|Get(acopy) (Variables|Default|GetDialogue_002) (Variables|Default|GetTalkIndex_002))))
          (Variables|/Game/ThirdPerson/Blueprints/BP_ThirdPersonCharacter.BP_ThirdPersonCharacter_C|SetTalkOver (Variables|Default|GetAs%20BP%20Third%20Person%20Character) true)
          (Variables|/Script/Engine.Character|SetJumpMaxCount (Variables|Default|GetAs%20BP%20Third%20Person%20Character) 0)
          (else
            (Variables|/Game/ThirdPerson/Blueprints/BP_ThirdPersonCharacter.BP_ThirdPersonCharacter_C|SetTalkOver (Variables|Default|GetAs%20BP%20Third%20Person%20Character) false :!label _label)
            (Variables|/Script/Engine.Character|SetJumpMaxCount (Variables|Default|GetAs%20BP%20Third%20Person%20Character) 2)
            (if (not (Variables|/Game/ThirdPerson/Blueprints/BP_ThirdPersonCharacter.BP_ThirdPersonCharacter_C|GetTimerStart (Variables|Default|GetAs%20BP%20Third%20Person%20Character)))
              (Utilities|FlowControl|Sequence
                (:then_0
                  (Transformation|SetActorLocation (Variables|Default|GetAs%20BP%20Third%20Person%20Character) "-3619.000000,-3643.000000,112.084760" false true))
                (:then_1
                  (Transformation|SetActorRotation (Variables|Default|GetAs%20BP%20Third%20Person%20Character) "0.000000,30.000000,0.000000")
                  (bind _returnvalue_2 (UserInterface|CreateWidget "/Game/SP_MJ_ALL/SP_UI/SP_GameUI/WB_CountDown.WB_CountDown_C"))
                  (UserInterface|Viewport|AddtoViewport _returnvalue_2 0)
                  (Variables|/Game/ThirdPerson/Blueprints/BP_ThirdPersonCharacter.BP_ThirdPersonCharacter_C|SetTimerStart (Variables|Default|GetAs%20BP%20Third%20Person%20Character) true)
                  (Input|DisableInput (Variables|Default|GetAs%20BP%20Third%20Person%20Character) 0)
                  (Widget|RemovefromParent (Variables|Default|GetUI))
                  (Variables|/Game/ThirdPerson/Blueprints/BP_ThirdPersonCharacter.BP_ThirdPersonCharacter_C|SetTalkagain (Variables|Default|GetAs%20BP%20Third%20Person%20Character) false))))))))
    (else
      (Math|Integer|IncrementInt (Variables|Default|GetTalkIndex)
        (:%20%20
          (if (< (Variables|Default|GetTalkIndex) (Utilities|Array|Length (Variables|Default|Getdialogue)))
            (Variables|Default|GetUI
              (:then
                _)
              (:else
                (bind _returnvalue_3 (Game|ConstructObjectfromClass (Game|GetPlayerController 0) "/Game/SP_MJ_ALL/SP_UI/SP_GameUI/WB_Dialogue_Frog.WB_Dialogue_Frog_C"))
                (bind _output_get_3 (Variables|Default|SetUI _returnvalue_3))
                (UserInterface|Viewport|AddtoViewport _output_get_3 0)))
            (Rendering|Components|TextRender|SetText (Variables|/Game/SP_MJ_ALL/SP_UI/SP_GameUI/WB_Dialogue_Frog.WB_Dialogue_Frog_C|GetTalkText (Variables|Default|GetUI)) (Utilities|Text|ToText(String) (Utilities|Array|Get(acopy) (Variables|Default|Getdialogue) (Variables|Default|GetTalkIndex))))
            (Variables|/Game/ThirdPerson/Blueprints/BP_ThirdPersonCharacter.BP_ThirdPersonCharacter_C|SetTalkOver (Variables|Default|GetAs%20BP%20Third%20Person%20Character) true)
            (Variables|/Script/Engine.Character|SetJumpMaxCount (Variables|Default|GetAs%20BP%20Third%20Person%20Character) 0)
            (Variables|/Game/ThirdPerson/Blueprints/BP_ThirdPersonCharacter.BP_ThirdPersonCharacter_C|SetStart (Variables|Default|GetAs%20BP%20Third%20Person%20Character) true)
            (else
              (goto _label))))))))

(fn ConstructionScript)
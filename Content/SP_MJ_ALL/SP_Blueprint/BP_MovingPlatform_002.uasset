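; BP_MovingPlatform_002 is a moving platform that travels along a straight line set by its Arrow component.
; On BeginPlay it stores its starting location and plays a timeline.
; Each update offsets that location along the Arrow's forward vector by the timeline's Move value times MoveDis.
; The location is set directly, without sweeping for collisions.
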(event EventBeginPlay
  (Variables|Default|SetFirstLocation (Transformation|GetActorLocation))
  (bind _move (Timeline|타임라인 Play)
    (:Update
      (Transformation|SetActorLocation (+ (Variables|Default|GetFirstLocation) (* (Math|Vector|GetForwardVector (Variables|Default|GetArrow)) (* _move (Variables|Default|GetMoveDis)))) false false))))

(fn ConstructionScript)
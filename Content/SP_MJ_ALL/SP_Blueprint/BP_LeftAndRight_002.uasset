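; BP_LeftAndRight_002 is an actor that slides back and forth or along a line from its starting position, likely a moving platform or obstacle.
; On BeginPlay it stores its location, sets the timeline play rate from PlayTime, and starts the timeline after DelayTime.
; Each timeline update offsets the actor along the Arrow component's forward vector by the track value times MoveDis, without sweeping.
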(event EventBeginPlay
  (Variables|Default|SetFirstLocation (Transformation|GetActorLocation))
  (Components|Timeline|SetPlayRate (Variables|Default|Get타임라인) (Variables|Default|GetPlayTime))
  (Utilities|FlowControl|Delay (Variables|Default|GetDelayTime))
  (bind _새_트랙_0 (Timeline|타임라인 Play)
    (:Update
      (Transformation|SetActorLocation (+ (Variables|Default|GetFirstLocation) (* (Math|Vector|GetForwardVector (Variables|Default|GetArrow)) (* _새_트랙_0 (Variables|Default|GetMoveDis)))) false false))))

(fn ConstructionScript)
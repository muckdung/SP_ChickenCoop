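; BP_Wheel is a one-time wheel pickup that triggers the game mode's RandomPart when its Box is overlapped, without checking what overlapped it.
; It then destroys the Box and mesh components, leaving the actor itself alive.
; A sequence also shows a LogUI widget on screen and removes it after a short delay.
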(event OnComponentBeginOverlap(Box)
  (params (OverlappedComponent :type Primitive%20Component%20Object%20Reference) (OtherActor :type Actor%20Object%20Reference) (OtherComp :type Primitive%20Component%20Object%20Reference) (OtherBodyIndex :type Integer) (bFromSweep :type Boolean) (SweepResult :type Hit%20Result%20Structure%20%28by%20ref%29))
  (Utilities|FlowControl|Sequence
    (:then_0
      (bind _asbp_third_person_game_mode (Utilities|Casting|CastToBP_ThirdPersonGameMode (Game|GetGameMode)))
      (Default|RandomPart _asbp_third_person_game_mode)
      (Components|DestroyComponent (Variables|Default|GetBox))
      (Components|DestroyComponent (Variables|Debug|GetStaticMeshComponent)))
    (:then_1
      (bind _returnvalue (UserInterface|CreateWidget "/Game/SP_MJ_ALL/SP_UI/SP_GameUI/LogUI.LogUI_C"))
      (UserInterface|Viewport|AddtoViewport _returnvalue 0)
      (Utilities|FlowControl|Delay 2.0)
      (Widget|RemovefromParent _returnvalue))))

(fn ConstructionScript)